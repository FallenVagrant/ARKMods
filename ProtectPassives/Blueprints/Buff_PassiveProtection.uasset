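; ARK dino buff that protects passive dinos near the Protection_Pillar that applied it, making them undamageable and unrideable.
; On start it checks nearby structures for that pillar, then runs timers that recheck proximity and passivity, destroying itself on failure, and drop eggs and certain non-food inventory items.
; It also blocks gas-maskable buffs and zeroes one torpor-poison damage type.
; Destruction re-enables damage and restores riding from the class default.
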(event Custom|CheckInventory2
  (Utilities|IsValid (Variables|/Script/ShooterGame.PrimalCharacter|GetMyInventoryComponent (stale EventBeginPlay _asprimaldinocharacter))
    (:Is%20Valid
      (Development|PrintString "Checking Inventory")
      (for _array_element (Variables|/Script/ShooterGame.PrimalInventoryComponent|GetInventoryItems (Variables|/Script/ShooterGame.PrimalCharacter|GetMyInventoryComponent (stale EventBeginPlay _asprimaldinocharacter)))
        (Utilities|Casting|CastToPrimalItemConsumable_Egg _array_element
          (:then
            (Class|PrimalInventoryComponent|RemoveItem (Variables|/Script/ShooterGame.PrimalCharacter|GetMyInventoryComponent (stale EventBeginPlay _asprimaldinocharacter)) (Variables|/Script/ShooterGame.PrimalItem|GetItemID _array_element) true false false true :!label _label))
          (:CastFailed
            (Utilities|Casting|CastToPrimalItemConsumableEatable _array_element
              (:CastFailed
                (bind _asprimalitem_base_c (Utilities|Casting|CastToPrimalItem_Base _array_element)
                  (:then
                    (if (not (and (< (Variables|/Script/ShooterGame.PrimalItem|GetItemRating _asprimalitem_base_c) 1.0) (Variables|/Script/ShooterGame.PrimalItem|GetbIsBlueprint _asprimalitem_base_c)))
                      (goto _label)))
                  (:CastFailed
                    (bind _asprimalitem_dye (Utilities|Casting|CastToPrimalItem_Dye _array_element)
                      (:then
                        (if (not (and (< (Variables|/Script/ShooterGame.PrimalItem|GetItemRating _asprimalitem_dye) 1.0) (Variables|/Script/ShooterGame.PrimalItem|GetbIsBlueprint _asprimalitem_dye)))
                          (goto _label)))
                      (:CastFailed
                        (bind _asprimalitem_radio (Utilities|Casting|CastToPrimalItem_Radio _array_element))
                        (if (not (and (< (Variables|/Script/ShooterGame.PrimalItem|GetItemRating _asprimalitem_radio) 1.0) (Variables|/Script/ShooterGame.PrimalItem|GetbIsBlueprint _asprimalitem_radio)))
                          (goto _label))))))))))))))

(event Custom|CheckDinoRadius
  (bind _pillarthatbuffed (Variables|Default|GetPillarThatBuffed))
  (Development|PrintString "Checking dino radius")
  (bind _asprimaldinocharacter (Utilities|Casting|CastToPrimalDinoCharacter (Variables|Default|GetInstigator)))
  (bind _returnvalue (Class|VictoryCore|ServerOctreeOverlapActors (Class|Actor|GetWorld _asprimaldinocharacter) (Transformation|GetActorLocation _asprimaldinocharacter) (Variables|/Game/Mods/ProtectPassives/Blueprints/Protection_Pillar.Protection_Pillar_C|GetStructureRadius _pillarthatbuffed) "STRUCTURES"))
  (bind _array_element (Utilities|Array|ForEachLoopwithBreak _returnvalue :!label _label)
    (:LoopBody
      (bind _asprotection_pillar_c (Utilities|Casting|CastToProtection_Pillar _array_element))
      (if (and (== _asprotection_pillar_c _pillarthatbuffed) (== (Variables|/Script/ShooterGame.PrimalDinoCharacter|GetTamedAggressionLevel _asprimaldinocharacter) 0))
        (Development|PrintString "Pillar still close")
        (goto _label Break)
        (else
          (Development|PrintString "Radius about to kill buff")
          (Actor|DestroyActor)
          (Development|PrintString "Radius Buff Dead"))))))

(event Custom|CheckInventory1
  (Utilities|IsValid (Variables|/Script/ShooterGame.PrimalCharacter|GetMyInventoryComponent (stale EventBeginPlay _asprimaldinocharacter_2))
    (:Is%20Valid
      (Development|PrintString "Checking Inventory")
      (for _array_element (Variables|/Script/ShooterGame.PrimalInventoryComponent|GetInventoryItems (Variables|/Script/ShooterGame.PrimalCharacter|GetMyInventoryComponent (stale EventBeginPlay _asprimaldinocharacter_2)))
        (Utilities|Casting|CastToPrimalItemConsumable_Egg _array_element
          (:then
            (Class|PrimalInventoryComponent|RemoveItem (Variables|/Script/ShooterGame.PrimalCharacter|GetMyInventoryComponent (stale EventBeginPlay _asprimaldinocharacter_2)) (Variables|/Script/ShooterGame.PrimalItem|GetItemID _array_element) true false false true :!label _label))
          (:CastFailed
            (Utilities|Casting|CastToPrimalItemConsumableEatable _array_element
              (:CastFailed
                (bind _asprimalitem_base_c (Utilities|Casting|CastToPrimalItem_Base _array_element)
                  (:then
                    (if (not (and (< (Variables|/Script/ShooterGame.PrimalItem|GetItemRating _asprimalitem_base_c) 1.0) (Variables|/Script/ShooterGame.PrimalItem|GetbIsBlueprint _asprimalitem_base_c)))
                      (goto _label)))
                  (:CastFailed
                    (bind _asprimalitem_dye (Utilities|Casting|CastToPrimalItem_Dye _array_element)
                      (:then
                        (if (not (and (< (Variables|/Script/ShooterGame.PrimalItem|GetItemRating _asprimalitem_dye) 1.0) (Variables|/Script/ShooterGame.PrimalItem|GetbIsBlueprint _asprimalitem_dye)))
                          (goto _label)))
                      (:CastFailed
                        (bind _asprimalitem_radio (Utilities|Casting|CastToPrimalItem_Radio _array_element))
                        (if (not (and (< (Variables|/Script/ShooterGame.PrimalItem|GetItemRating _asprimalitem_radio) 1.0) (Variables|/Script/ShooterGame.PrimalItem|GetbIsBlueprint _asprimalitem_radio)))
                          (goto _label))))))))))))))

(event Custom|DisableRiding
  (Variables|/Script/ShooterGame.PrimalDinoCharacter|SetbAllowRiding (stale EventBeginPlay _asprimaldinocharacter_2) false))

(event EventBeginPlay
  (bind _pillarthatbuffed (Variables|Default|GetPillarThatBuffed))
  (bind _protbufficon (Variables|Default|GetProtBuffIcon))
  (bind _protbufficon_2 (Variables|Default|GetProtBuffIcon))
  (bind _instigator (Variables|Default|GetInstigator))
  (Utilities|FlowControl|Delay 1.0)
  (if (Variables|Default|GetBuffApplied)
    (bind _asprimaldinocharacter (Utilities|Casting|CastToPrimalDinoCharacter _instigator))
    (if (Variables|/Script/ShooterGame.PrimalCharacter|GetbIsBigDino _asprimaldinocharacter)
      (Transformation|SetRelativeScale3D _protbufficon_2 "1.700000,1.700000,1.700000")
      (Transformation|SetRelativeLocation _protbufficon_2 "0, 0,15.000000" false))
    (if (Variables|Default|GetHideIcon)
      (Development|SetHiddeninGame _protbufficon_2 true false)
      (else
        (Development|SetHiddeninGame _protbufficon_2 false false)))
    (Development|PrintString "Buffing")
    (if (Variables|/Script/ShooterGame.PrimalDinoCharacter|GetbHasRider _asprimaldinocharacter)
      (Class|PrimalDinoCharacter|ForceClearRider _asprimaldinocharacter))
    (Variables|/Script/ShooterGame.PrimalDinoCharacter|SetbAllowRiding _asprimaldinocharacter false)
    (Variables|/Script/Engine.Actor|SetbCanBeDamaged _asprimaldinocharacter false false)
    (Variables|Default|SetBuffApplied true false)
    (Utilities|Time|SetTimerbyFunctionName 0 "CheckInventory2" 5.0 true)
    (Utilities|Time|SetTimerbyFunctionName 0 "CheckDinoRadius" 1e+01 true)
    (else
      (Development|PrintString (Utilities|String|Append "Buffing Pillar: " (Utilities|GetDisplayName _pillarthatbuffed)))
      (bind _asprimaldinocharacter_2 (Utilities|Casting|CastToPrimalDinoCharacter _instigator))
      (Development|PrintString (Utilities|String|Append "Dino: " (Utilities|GetDisplayName _instigator)))
      (Utilities|FlowControl|Delay (Variables|Default|GetDelay))
      (if (Variables|/Script/ShooterGame.PrimalCharacter|GetbIsBigDino _asprimaldinocharacter_2)
        (Transformation|SetRelativeScale3D _protbufficon "1.500000,1.500000,1.500000")
        (Transformation|SetRelativeLocation _protbufficon "0, 0,15.000000" false))
      (if (Variables|Default|GetHideIcon)
        (Development|SetHiddeninGame _protbufficon true false)
        (else
          (Development|SetHiddeninGame _protbufficon false false)))
      (bind _returnvalue (Class|VictoryCore|ServerOctreeOverlapActors (Class|Actor|GetWorld _asprimaldinocharacter_2) (Transformation|GetActorLocation _asprimaldinocharacter_2) (Variables|/Game/Mods/ProtectPassives/Blueprints/Protection_Pillar.Protection_Pillar_C|GetStructureRadius _pillarthatbuffed) "STRUCTURES"))
      (bind _array_element (Utilities|Array|ForEachLoopwithBreak _returnvalue :!label _label)
        (:LoopBody
          (bind _asprotection_pillar_c (Utilities|Casting|CastToProtection_Pillar _array_element))
          (Development|SetHiddeninGame _protbufficon false false)
          (if (and (== _asprotection_pillar_c (Variables|Default|GetPillarThatBuffed)) (== (Variables|/Script/ShooterGame.PrimalDinoCharacter|GetTamedAggressionLevel _asprimaldinocharacter_2) 0))
            (Variables|Default|SetStillBuffed true false)
            (else
              (Variables|Default|SetStillBuffed false false)))
          (if (Variables|Default|GetStillBuffed)
            (if (Variables|/Script/ShooterGame.PrimalDinoCharacter|GetbHasRider _asprimaldinocharacter_2)
              (Class|PrimalDinoCharacter|ForceClearRider _asprimaldinocharacter_2))
            (CallFunction|DisableRiding)
            (Variables|/Script/Engine.Actor|SetbCanBeDamaged _asprimaldinocharacter_2 false false)
            (Variables|Default|SetBuffApplied true false)
            (Utilities|Time|SetTimerbyFunctionName 0 "CheckInventory1" 5.0 true)
            (Utilities|Time|SetTimerbyFunctionName 0 "CheckDinoRadius" 1e+01 true)
            (goto _label Break)
            (else
              (Development|PrintString "Don't buff")
              (Development|SetHiddeninGame (Variables|Default|GetProtBuffIcon) true false)
              (Development|PrintString "About to destroy buff")
              (Actor|DestroyActor)
              (Development|PrintString "Buff Dead"))))))))

(event EventDestroyed
  (Development|PrintString "Start Buff Destroy")
  (bind _asprimaldinocharacter (Utilities|Casting|CastToPrimalDinoCharacter (Variables|Default|GetInstigator)))
  (bind _returnvalue (Class|VictoryCore|GetClassDefaultObject (Utilities|GetClass _asprimaldinocharacter)))
  (bind _asprimaldinocharacter_2 (Utilities|Casting|CastToPrimalDinoCharacter _returnvalue))
  (Variables|/Script/ShooterGame.PrimalDinoCharacter|SetbAllowRiding _asprimaldinocharacter (Variables|/Script/ShooterGame.PrimalDinoCharacter|GetbAllowRiding _asprimaldinocharacter_2))
  (Development|PrintString "Allowed to Ride")
  (Variables|/Script/Engine.Actor|SetbCanBeDamaged _asprimaldinocharacter true false)
  (Development|PrintString "Can be damaged")
  (Variables|Default|SetStillBuffed false false)
  (Development|PrintString "Buff Destroyed")
  (Variables|Default|SetBuffApplied false false)
  (Development|SetHiddeninGame (Variables|Default|GetProtBuffIcon) true false)
  (Class|PrimalBuff|BPDeactivate)
  (Development|PrintString "Buff Dead"))

(fn ConstructionScript)

(fn BPPreventAddingOtherBuff
  (params (anotherBuffClass :type Primal%20Buff%20Class%20Reference))
  (LocalVariables|SetretVal false)
  (Utilities|Casting|CastToBuff_Base_Disease_Low_GasMaskableClass anotherBuffClass
    (:then
      (LocalVariables|SetretVal true :!label _label))
    (:CastFailed
      (Utilities|Casting|CastToBuff_Base_GasMaskableClass anotherBuffClass
        (:then
          (goto _label))
        (:CastFailed
          _))))
  (return (LocalVariables|GetretVal)))

(fn BuffAdjustDamage
  (params (Damage :type Float%20%28single-precision%29) (HitInfo :type Hit%20Result%20Structure%20%28by%20ref%29) (EventInstigator :type Controller%20Object%20Reference) (DamageCauser :type Actor%20Object%20Reference) (TheDamgeType :type Damage%20Type%20Class%20Reference))
  (LocalVariables|SetretVal Damage)
  (Utilities|Casting|CastToDmgType_Melee_TorpPoison_Large_NoFFClass TheDamgeType
    (:then
      (LocalVariables|SetretVal 0.0))
    (:CastFailed
      _))
  (return (LocalVariables|GetretVal)))