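; A test structure that adds a "Set TextRender" multi-use entry, letting players set the text on its text render component.
; Selecting the entry creates a UI_TextInput widget on the client and hands it a reference to the structure.
; An "Update Text Render" net exec command stores the submitted string in CurrentText on the server and forces a net update.
; The RepNotify on CurrentText then applies it to the component.
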(event EventBPClientDoMultiUse
  (params (ForPC :type Player%20Controller%20Object%20Reference) (ClientUseIndex :type Integer))
  ;[1 1 1] BPClient Do Multi Use - Perform actions on the client when a multiuse entry is selected
  ;;[0.05112 1 0.05112] Start
  ;;[0.05112 1 0.05112] Perform actions for the selected "Use String"
  (switch int ClientUseIndex
    (:9001
      ;;[1 1 1] Create the Input Widget
      (bind _returnvalue (UserInterface|CreateWidget "/Game/Mods/ProtectPassives/Widgets/UI_TextInput.UI_TextInput_C" ForPC))
      ;;[1 1 1] Set reference to self on Input Widget
      (Variables|/Game/Mods/ProtectPassives/Widgets/UI_TextInput.UI_TextInput_C|SetStructure _returnvalue self)
      ;;[1 1 1] Add Widget to Viewport
      (UserInterface|Viewport|AddtoViewport _returnvalue))))

(fn ConstructionScript)

(fn BPTryMultiUse
  (params (ForPC :type Player%20Controller%20Object%20Reference) (UseIndex :type Integer))
  ;[1 1 1] BPTry Multi Use - Perform actions when a menu entry is activated
  ;;[0.05112 1 0.05112] Start
  ;;[0.05112 1 0.05112] Return Node
  (return true))

(fn BPGetMultiUseEntries
  (params (ForPC :type Player%20Controller%20Object%20Reference) (MultiUseEntries :type Array%20of%20Multi%20Use%20Entry%20Structures))
  ;[1 1 1] BPGet Multi Use - Hook into the MultiUse array to add to or edit the default MultiUse Entries
  ;;[0.05112 1 0.05112] Start
  ;;[0.05112 1 0.05112] Saving the incoming MultiUse Entry array to temporay variable
  (LocalVariables|SetReturnUseEntries MultiUseEntries)
  ;;[0.05112 1 0.05112] Adding our custom MultiUse Entry to the temporary array
  (Utilities|Array|Add (LocalVariables|GetReturnUseEntries) (Utilities|Struct|MakeMultiUseEntry 0 "Set TextRender" 9001 0 false false false false true))
  ;;[0.05112 1 0.05112] Setting the "Return Value" to the temporary array
  (return (LocalVariables|GetReturnUseEntries)))

(fn BPServerHandleNetExecCommand
  (params (FromPC :type Player%20Controller%20Object%20Reference) (CommandName :type Name :default "None") (ExecParams :type BP%20Net%20Exec%20Params%20Structure%20%28by%20ref%29))
  ;[1 1 1] Check for Update Text Render Command
  (switch name CommandName
    (:Default
      _)
    (:UpdateTextRender
      ;[1 1 1] Set "Current Text" to input text(Calls "On Rep Current Text")
      (Variables|Default|SetCurrentText (.StringParam1 (Utilities|Struct|BreakBPNetExecParams ExecParams)) false)
      ;[1 1 1] ForceReplication
      (Networking|ForceNetUpdate)))
  (return false))

(fn OnRepCurrentText
  ;[1 1 1] Set Current Text to Text Render Component
  (Rendering|Components|TextRender|SetText (Variables|Default|GetTheTextRenderComponent) (Variables|Default|GetCurrentText)))