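; Placeable tribe structure that gives Buff_PassiveProtection to same-team tamed dinos set to passive within its radius.
; A looping server timer clamps the INI-limited radius, enforces the tribe pillar cap and octree-scans dinos to add or remove buffs.
; Each buff records its source pillar, which alone removes it on sphere exit or destruction.
; Multi-use entries open the radius menu or toggle sphere visibility; radius changes arrive by net exec and replicate via OnRep.
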(event OnComponentEndOverlap(AoE)
  (params (OtherActor :type Actor%20Object%20Reference) (OtherComp :type Primitive%20Component%20Object%20Reference) (OtherBodyIndex :type Integer))
  ;[1 1 1] Exiting Sphere
  (bind _asprimaldinocharacter (Utilities|Casting|CastToPrimalDinoCharacter OtherActor)
    (:then
      (Development|PrintString "Dino End Overlap")
      (if (== (Variables|/Script/Engine.Actor|GetTargetingTeam _asprimaldinocharacter) (Variables|Default|GetTargetingTeam))
        (bind _returnvalue (Class|PrimalCharacter|HasBuff _asprimaldinocharacter "/Game/Mods/ProtectPassives/Blueprints/Buff_PassiveProtection.Buff_PassiveProtection_C" false))
        (if _returnvalue
          (bind _returnvalue_2 (Class|PrimalCharacter|GetBuff _asprimaldinocharacter "/Game/Mods/ProtectPassives/Blueprints/Buff_PassiveProtection.Buff_PassiveProtection_C"))
          (bind _asbuff_passiveprotection_c (Utilities|Casting|CastToBuff_PassiveProtection _returnvalue_2))
          (if (== (Variables|/Game/Mods/ProtectPassives/Blueprints/Buff_PassiveProtection.Buff_PassiveProtection_C|GetPillarThatBuffed _asbuff_passiveprotection_c) self)
            (Class|PrimalCharacter|DeactivateBuffs _asprimaldinocharacter "/Game/Mods/ProtectPassives/Blueprints/Buff_PassiveProtection.Buff_PassiveProtection_C" 0 false)
            (Development|PrintString "Buff Removed" :!label _label)))))
    (:CastFailed
      (bind _asshootercharacter (Utilities|Casting|CastToShooterCharacter OtherActor))
      (if (== (Variables|/Script/Engine.Actor|GetTargetingTeam (Variables|/Script/ShooterGame.PrimalCharacter|GetMountedDino _asshootercharacter)) (Variables|Default|GetTargetingTeam))
        (bind _returnvalue_3 (Class|PrimalCharacter|HasBuff (Variables|/Script/ShooterGame.PrimalCharacter|GetMountedDino _asshootercharacter) "/Game/Mods/ProtectPassives/Blueprints/Buff_PassiveProtection.Buff_PassiveProtection_C" false))
        (if _returnvalue_3
          (bind _returnvalue_4 (Class|PrimalCharacter|GetBuff (Variables|/Script/ShooterGame.PrimalCharacter|GetMountedDino _asshootercharacter) "/Game/Mods/ProtectPassives/Blueprints/Buff_PassiveProtection.Buff_PassiveProtection_C"))
          (bind _asbuff_passiveprotection_c_2 (Utilities|Casting|CastToBuff_PassiveProtection _returnvalue_4))
          (if (== (Variables|/Game/Mods/ProtectPassives/Blueprints/Buff_PassiveProtection.Buff_PassiveProtection_C|GetPillarThatBuffed _asbuff_passiveprotection_c_2) self)
            (Class|PrimalCharacter|DeactivateBuffs (Variables|/Script/ShooterGame.PrimalCharacter|GetMountedDino _asshootercharacter) "/Game/Mods/ProtectPassives/Blueprints/Buff_PassiveProtection.Buff_PassiveProtection_C" 0 false)
            (goto _label)))))))

(event Custom|CheckRadius
  (bind _structuremaxradius (Variables|Default|GetStructureMaxRadius))
  (bind _tribepillars (Variables|Default|GetTribePillars))
  (bind _returnvalue (Utilities|Array|Length _tribepillars))
  ;[1 1 1] Evaluate radius and give buff
  (if (not (Variables|Default|GetEvaluating))
    (Development|PrintString "Checking")
    (Utilities|Array|Clear (Variables|Default|GetTribePillars))
    (Variables|Default|SetEvaluating true)
    (if (>= (Variables|Default|GetStructureRadius) _structuremaxradius)
      (Variables|Default|SetStructureRadius _structuremaxradius false)
      (Networking|ForceNetUpdate)
      (Networking|ForceNetUpdate :!label _label)
      (else
        (bind _outactors (Actor|GetAllActorsOfClass "Protection_Pillar_C"))
        (for _array_element _outactors
          (if (== (Variables|/Script/Engine.Actor|GetTargetingTeam _array_element) (Variables|Default|GetTargetingTeam))
            (if (Utilities|Array|ContainsItem _tribepillars _array_element)
              _
              (else
                (Utilities|Array|Add _tribepillars _array_element)))
            (Development|PrintString (Utilities|String|BuildString(Integer) "" "Tribe pillars: " _returnvalue))
            (if (> _returnvalue (Variables|Default|GetMaxStructures))
              (bind _asprotection_pillar_c (Utilities|Casting|CastToProtection_Pillar (Utilities|Array|Get(acopy) _tribepillars (- _returnvalue 1))))
              (Actor|DestroyActor _asprotection_pillar_c)
              (Utilities|Array|RemoveItem _tribepillars _array_element)
              (goto _label)
              (else
                (goto _label)))
            (else
              (goto _label))))
        (Variables|Default|SetEvaluating false)))
    (bind _returnvalue_2 (Class|VictoryCore|ServerOctreeOverlapActors (Class|Actor|GetWorld) (Transformation|GetActorLocation) (Variables|Default|GetStructureRadius) "DINOPAWNS_TAMED"))
    (Development|PrintString (Utilities|String|Append "Dinos In Sphere: " (Utilities|String|ToString(Integer) (Utilities|Array|Length _returnvalue_2))))
    (for _array_element_2 _returnvalue_2
      (bind _asprimaldinocharacter (Utilities|Casting|CastToPrimalDinoCharacter _array_element_2))
      (if (== (Variables|/Script/Engine.Actor|GetTargetingTeam _asprimaldinocharacter) (Variables|Default|GetTargetingTeam))
        (if (== (Variables|/Script/ShooterGame.PrimalDinoCharacter|GetTamedAggressionLevel _asprimaldinocharacter) 0)
          (bind _returnvalue_3 (Class|PrimalCharacter|HasBuff _asprimaldinocharacter "/Game/Mods/ProtectPassives/Blueprints/Buff_PassiveProtection.Buff_PassiveProtection_C" false))
          (if _returnvalue_3
            (Development|PrintString "Apparently, already has the buff")
            (else
              (bind _returnvalue_4 (Class|PrimalBuff|StaticAddBuff "/Game/Mods/ProtectPassives/Blueprints/Buff_PassiveProtection.Buff_PassiveProtection_C" _asprimaldinocharacter 0 0 true))
              (bind _asbuff_passiveprotection_c (Utilities|Casting|CastToBuff_PassiveProtection _returnvalue_4))
              (Variables|/Game/Mods/ProtectPassives/Blueprints/Buff_PassiveProtection.Buff_PassiveProtection_C|SetPillarThatBuffed _asbuff_passiveprotection_c self false)
              (Variables|/Game/Mods/ProtectPassives/Blueprints/Buff_PassiveProtection.Buff_PassiveProtection_C|SetDelay _asbuff_passiveprotection_c (Variables|Default|GetBuffDelay) false)
              (Variables|/Game/Mods/ProtectPassives/Blueprints/Buff_PassiveProtection.Buff_PassiveProtection_C|SetHideIcon _asbuff_passiveprotection_c (Variables|Default|GetHideBuffIcon) false)))
          (else
            (bind _returnvalue_5 (Class|PrimalCharacter|HasBuff _asprimaldinocharacter "/Game/Mods/ProtectPassives/Blueprints/Buff_PassiveProtection.Buff_PassiveProtection_C" false :!label _label_2))
            (if _returnvalue_5
              (bind _returnvalue_6 (Class|PrimalCharacter|GetBuff _asprimaldinocharacter "/Game/Mods/ProtectPassives/Blueprints/Buff_PassiveProtection.Buff_PassiveProtection_C"))
              (bind _asbuff_passiveprotection_c_2 (Utilities|Casting|CastToBuff_PassiveProtection _returnvalue_6))
              (if (== (Variables|/Game/Mods/ProtectPassives/Blueprints/Buff_PassiveProtection.Buff_PassiveProtection_C|GetPillarThatBuffed _asbuff_passiveprotection_c_2) self)
                (Class|PrimalCharacter|DeactivateBuffs _asprimaldinocharacter "/Game/Mods/ProtectPassives/Blueprints/Buff_PassiveProtection.Buff_PassiveProtection_C" 0 false)
                (Development|PrintString "Buff Removed")
                (Variables|/Game/Mods/ProtectPassives/Blueprints/Buff_PassiveProtection.Buff_PassiveProtection_C|SetPillarThatBuffed _asbuff_passiveprotection_c_2 0 false)))))
        (else
          (goto _label_2))))
    (Variables|Default|SetEvaluating false)))

(event EventBPClientDoMultiUse
  (params (ForPC :type Player%20Controller%20Object%20Reference) (ClientUseIndex :type Integer))
  (bind _structuremaxradius (Variables|Default|GetStructureMaxRadius))
  (bind _aoe (Variables|Default|GetAoE))
  ;[1 1 1] MultiUse
  (switch int ClientUseIndex
    (:33446
      (bind _returnvalue (UserInterface|CreateWidget "/Game/Mods/ProtectPassives/Widgets/Protection_Menu.Protection_Menu_C" ForPC))
      (Variables|/Game/Mods/ProtectPassives/Widgets/Protection_Menu.Protection_Menu_C|SetStructure _returnvalue self)
      (Variables|/Game/Mods/ProtectPassives/Widgets/Protection_Menu.Protection_Menu_C|SetRadius _returnvalue (Variables|Default|GetStructureRadius) false)
      (Variables|/Game/Mods/ProtectPassives/Widgets/Protection_Menu.Protection_Menu_C|SetMaxRadius _returnvalue _structuremaxradius false)
      (Class|SpinBox|SetMaxSliderValue (Variables|/Game/Mods/ProtectPassives/Widgets/Protection_Menu.Protection_Menu_C|GetRadiusSpinBox _returnvalue) _structuremaxradius)
      (Class|SpinBox|SetMaxValue (Variables|/Game/Mods/ProtectPassives/Widgets/Protection_Menu.Protection_Menu_C|GetRadiusSpinBox _returnvalue) _structuremaxradius)
      (UserInterface|Viewport|AddtoViewport _returnvalue))
    (:33447
      (if (Variables|/Script/Engine.SceneComponent|GetbHiddenInGame _aoe)
        (Development|SetHiddeninGame _aoe false false)
        (else
          (Development|SetHiddeninGame _aoe true false))))))

(event EventDestroyed
  ;[1 1 1] On Pillar Pickup/Destroy
  (Utilities|SwitchNetAuthority
    (:DedicatedServer
      _)
    (:PlayerServer
      _))
  (Development|PrintString "Noooooo!")
  (bind _returnvalue (Class|VictoryCore|ServerOctreeOverlapActors (Class|Actor|GetWorld) (Transformation|GetActorLocation) (Variables|Default|GetStructureRadius) "DINOPAWNS_TAMED"))
  (for _array_element _returnvalue
    (bind _asprimaldinocharacter (Utilities|Casting|CastToPrimalDinoCharacter _array_element))
    (if (== (Variables|/Script/Engine.Actor|GetTargetingTeam _asprimaldinocharacter) (Variables|Default|GetTargetingTeam))
      (bind _returnvalue_2 (Class|PrimalCharacter|HasBuff _asprimaldinocharacter "/Game/Mods/ProtectPassives/Blueprints/Buff_PassiveProtection.Buff_PassiveProtection_C" false))
      (if _returnvalue_2
        (bind _returnvalue_3 (Class|PrimalCharacter|GetBuff _asprimaldinocharacter "/Game/Mods/ProtectPassives/Blueprints/Buff_PassiveProtection.Buff_PassiveProtection_C"))
        (bind _asbuff_passiveprotection_c (Utilities|Casting|CastToBuff_PassiveProtection _returnvalue_3))
        (if (== (Variables|/Game/Mods/ProtectPassives/Blueprints/Buff_PassiveProtection.Buff_PassiveProtection_C|GetPillarThatBuffed _asbuff_passiveprotection_c) self)
          (Class|PrimalCharacter|DeactivateBuffs _asprimaldinocharacter "/Game/Mods/ProtectPassives/Blueprints/Buff_PassiveProtection.Buff_PassiveProtection_C" 0 false)
          (Development|PrintString "Buff Removed")
          (Variables|/Game/Mods/ProtectPassives/Blueprints/Buff_PassiveProtection.Buff_PassiveProtection_C|SetPillarThatBuffed _asbuff_passiveprotection_c 0 false))))))

(event EventBeginPlay
  ;[1 1 1] Evaluate radius and give buff
  (Utilities|FlowControl|Delay 0.5)
  (Networking|SwitchHasAuthority
    (:Authority
      (if (not (Variables|Default|GetbIsPreviewStructure))
        (Variables|Default|SetStructureRadius (Variables|Default|GetInitRadius) false)
        (Development|PrintString (Utilities|String|BuildString(Float) "" "AoE Radius: " (Variables|/Script/Engine.SphereComponent|GetSphereRadius (Variables|Default|GetAoE))))
        (bind _asshootergamemode (Utilities|Casting|CastToShooterGameMode (Game|GetGameMode)))
        (bind _returnvalue (Class|ShooterGameMode|GetFloatOptionIni _asshootergamemode "ProtectPassives" "PillarMaxRadius"))
        (Variables|Default|SetStructureMaxRadius _returnvalue false)
        (bind _returnvalue_2 (Class|ShooterGameMode|GetIntOptionIni _asshootergamemode "ProtectPassives" "TribeMaxPillars"))
        (Variables|Default|SetMaxStructures _returnvalue_2)
        (bind _returnvalue_3 (Class|ShooterGameMode|GetFloatOptionIni _asshootergamemode "ProtectPassives" "BuffDelay"))
        (Variables|Default|SetBuffDelay _returnvalue_3)
        (bind _returnvalue_4 (Class|ShooterGameMode|GetBoolOptionIni _asshootergamemode "ProtectPassives" "HideBuffIcon"))
        (Variables|Default|SetHideBuffIcon _returnvalue_4)
        (Utilities|Time|SetTimerbyFunctionName 0 "CheckRadius" 1.0 true)
        (Development|PrintString (Utilities|String|BuildString(Float) "" "Max Radius: " (Variables|Default|GetStructureMaxRadius)))
        (Development|PrintString (Utilities|String|BuildString(Integer) "" "Max Structures: " (Variables|Default|GetMaxStructures)))
        (Networking|ForceNetUpdate)))))

(fn ConstructionScript)

(fn BPGetMultiUseEntries
  (params (ForPC :type Player%20Controller%20Object%20Reference) (MultiUseEntries :type Array%20of%20Multi%20Use%20Entry%20Structures))
  (bind _returnvalue (Math|Conversions|ToColor(LinearColor) "(R=0.146971,G=0.890000,B=0.813361,A=1.000000)"))
  (Variables|Default|SetReturnUseEntries MultiUseEntries)
  (if (== (Variables|/Script/Engine.Actor|GetTargetingTeam ForPC) (Variables|Default|GetTargetingTeam))
    (bind _muentriesarrayout (CallFunction|MUPickupDelay (Variables|Default|GetReturnUseEntries)))
    (Variables|Default|SetReturnUseEntries _muentriesarrayout)
    (Utilities|Array|Add (Variables|Default|GetReturnUseEntries) (Utilities|Struct|MakeMultiUseEntry 0 "Protection Radius" 33446 -1005 false false false false false false false false false true false false 0 "(B=175,G=175,R=175,A=255)" _returnvalue))
    (Utilities|Array|Add (Variables|Default|GetReturnUseEntries) (Utilities|Struct|MakeMultiUseEntry 0 "Toggle Protection Radius Visibility" 33447 -1006 false false false false false false false false false true false false 0 "(B=175,G=175,R=175,A=255)" _returnvalue)))
  (return (Variables|Default|GetReturnUseEntries)))

(fn MUPickupDelay
  (params (MUEntriesArray :type Array%20of%20Multi%20Use%20Entry%20Structures))
  (bind (_array_element _array_index) (Utilities|Array|ForEachLoopwithBreak MUEntriesArray :!label _label)
    (:LoopBody
      (if (== (.UseIndex (Utilities|Struct|BreakMultiUseEntry _array_element)) 203)
        (Utilities|Array|SetArrayElem MUEntriesArray _array_index (Utilities|Struct|MakeMultiUseEntry (.ForComponent (Utilities|Struct|BreakMultiUseEntry (Utilities|Array|Get(acopy) MUEntriesArray _array_index))) (.UseString (Utilities|Struct|BreakMultiUseEntry (Utilities|Array|Get(acopy) MUEntriesArray _array_index))) (.UseIndex (Utilities|Struct|BreakMultiUseEntry (Utilities|Array|Get(acopy) MUEntriesArray _array_index))) -10001 (.bHideFromUI (Utilities|Struct|BreakMultiUseEntry (Utilities|Array|Get(acopy) MUEntriesArray _array_index))) (.bDisableUse (Utilities|Struct|BreakMultiUseEntry (Utilities|Array|Get(acopy) MUEntriesArray _array_index))) (.bHideActivationKey (Utilities|Struct|BreakMultiUseEntry (Utilities|Array|Get(acopy) MUEntriesArray _array_index))) (.bRepeatMultiUse (Utilities|Struct|BreakMultiUseEntry (Utilities|Array|Get(acopy) MUEntriesArray _array_index))) (.bDisplayOnInventoryUI (Utilities|Struct|BreakMultiUseEntry (Utilities|Array|Get(acopy) MUEntriesArray _array_index))) (.bDisplayOnInventoryUISecondary (Utilities|Struct|BreakMultiUseEntry (Utilities|Array|Get(acopy) MUEntriesArray _array_index))) (.bHarvestable (Utilities|Struct|BreakMultiUseEntry (Utilities|Array|Get(acopy) MUEntriesArray _array_index))) (.bIsSecondaryUse (Utilities|Struct|BreakMultiUseEntry (Utilities|Array|Get(acopy) MUEntriesArray _array_index))) (.bPersistWheelOnActivation (Utilities|Struct|BreakMultiUseEntry (Utilities|Array|Get(acopy) MUEntriesArray _array_index))) (.bOverrideUseTextColor (Utilities|Struct|BreakMultiUseEntry (Utilities|Array|Get(acopy) MUEntriesArray _array_index))) (.bDisplayOnInventoryUITertiary (Utilities|Struct|BreakMultiUseEntry (Utilities|Array|Get(acopy) MUEntriesArray _array_index))) false (.WheelCategory (Utilities|Struct|BreakMultiUseEntry (Utilities|Array|Get(acopy) MUEntriesArray _array_index))) (.DisableUseColor (Utilities|Struct|BreakMultiUseEntry (Utilities|Array|Get(acopy) MUEntriesArray _array_index))) (.UseTextColor (Utilities|Struct|BreakMultiUseEntry (Utilities|Array|Get(acopy) MUEntriesArray _array_index))) 1.0 1.0 (.ActivationSound (Utilities|Struct|BreakMultiUseEntry (Utilities|Array|Get(acopy) MUEntriesArray _array_index)))))
        (goto _label Break)))
    (:Completed
      (return MUEntriesArray))))

(fn BPTryMultiUse
  (params (ForPC :type Player%20Controller%20Object%20Reference) (UseIndex :type Integer))
  (if (== (Variables|/Script/Engine.Actor|GetTargetingTeam ForPC) (Variables|Default|GetTargetingTeam))
    (return true)))

(fn OnRepStructureRadius
  (bind _structureradius (Variables|Default|GetStructureRadius))
  (Components|Sphere|SetSphereRadius (Variables|Default|GetAoE) _structureradius true)
  (Variables|Default|SetInitRadius _structureradius false))

(fn BPServerHandleNetExecCommand
  (params (FromPC :type Player%20Controller%20Object%20Reference) (CommandName :type Name :default "None") (ExecParams :type BP%20Net%20Exec%20Params%20Structure%20%28by%20ref%29))
  (switch name CommandName
    (:Default
      _)
    (:UpdateRadius
      (Variables|Default|SetStructureRadius (.FloatParam1 (Utilities|Struct|BreakBPNetExecParams ExecParams)) false)
      (Networking|ForceNetUpdate)))
  (return false))

(fn OnRepDinosinRadiusSVR)